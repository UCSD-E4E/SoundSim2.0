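; BP_AudioQueuePlayer is an actor that loads WAV files from a folder at BeginPlay and plays them in sequence.
; Each OnAudioFinished event calls PlayNext, which advances through the queue on AudioComp.
; Before each track, Randomize teleports the actor by a stored X/Y offset, but its random-value assignments are unconnected.
; LoopQueue is forced false at queue end, so playback stops there instead of looping.
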(event `self.ReceiveBeginPlay`
  (bind _returnvalue (`self.LoadWavsFromFolder` (`self.AudioFolder`)))
  (set `self.Queue` _returnvalue)
  (`self.PlayNext`))

(event `PlayNext`
  (if (> (`KismetArrayLibrary.Array_Length` (`self.Queue`)) 0)
    (if (>= (`self.CurrentIndex`) (`KismetArrayLibrary.Array_Length` (`self.Queue`)))
      (bind _output_get (set `self.LoopQueue` false))
      (if _output_get
        (set `self.CurrentIndex` 0)
        (`self.Randomize` :!label _label)
        (`AudioComponent.SetSound` (`self.AudioComp`) (`|GetArrayItem` (`self.Queue`) (`self.CurrentIndex`)))
        (`AudioComponent.Play` (`self.AudioComp`) 0.0)
        (set `self.CurrentIndex` (+ (`self.CurrentIndex`) 1))
        (else
          (`AudioComponent.Stop` (`self.AudioComp`) :!label _label_2)))
      (else
        (goto _label)))
    (else
      (goto _label_2))))

(event `self.AudioComp.OnAudioFinished`
  (`self.PlayNext`))

(fn `Randomize`
  (`self.K2_SetActorLocation` (+ (`self.K2_GetActorLocation`) (`KismetMathLibrary.MakeVector` (`self.X`) (`self.Y`))) false true))

(fn `UserConstructionScript`)